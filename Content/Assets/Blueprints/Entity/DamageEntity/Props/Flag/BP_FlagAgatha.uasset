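; BP_FlagAgatha is a damageable flag prop that falls apart and drops studs when its health runs out.
; On destruction it turns on physics for the mesh pieces gathered by SetupMesh, ignores pawn collision and plays a random fall-apart sound.
; It then spawns a random number of BP_Stud pickups at its sphere, some with an alternate type, and removes itself after a short delay.
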(event Custom|DestroyObject
  (Variables|Default|SetIsDestroy true)
  (CallFunction|SetPhysics)
  (Audio|PlaySoundatLocation (Utilities|Select :Index (Math|Random|RandomIntegerinRange 0 4) :Option%200 "/Game/Assets/Audio/Build/Destroy/SW_FALLAPART01.SW_FALLAPART01" :Option%201 "/Game/Assets/Audio/Build/Destroy/SW_FALLAPART02.SW_FALLAPART02" :Option%202 "/Game/Assets/Audio/Build/Destroy/SW_FALLAPART03.SW_FALLAPART03" :Option%203 "/Game/Assets/Audio/Build/Destroy/SW_FALLAPART04.SW_FALLAPART04" :Option%204 "/Game/Assets/Audio/Build/Destroy/SW_FALLAPART05.SW_FALLAPART05") (Transformation|GetActorLocation) "0, 0, 0" 1.0 1.0 0.0 0 0 0 0)
  (CallFunction|SpawnStud)
  (Utilities|FlowControl|Delay 5.0)
  (Actor|DestroyActor))

(event Game|Damage|EventAnyDamage
  (params (Damage :type Float%20%28single-precision%29) (DamageType :type Damage%20Type%20Object%20Reference) (InstigatedBy :type Controller%20Object%20Reference) (DamageCauser :type Actor%20Object%20Reference))
  (Variables|Default|SetHealth (- (Variables|Default|GetHealth) Damage))
  (if (not (Variables|Default|GetIsDestroy))
    (if (<= (Variables|Default|GetHealth) 0.0)
      (CallFunction|DestroyObject))))

(event EventBeginPlay
  (Variables|Default|SetArrayMesh (Utilities|SetupMesh)))

(fn ConstructionScript)

(fn SetPhysics
  (bind _sphere (Variables|Default|GetSphere))
  (for _array_element (Variables|Default|GetArrayMesh)
    (Collision|SetCollisionResponsetoChannel _array_element "ECC_Pawn" "ECR_Ignore")
    (Physics|SetSimulatePhysics _array_element true))
  (Collision|SetCollisionEnabled _sphere "QueryAndPhysics")
  (Collision|SetCollisionResponsetoChannel _sphere "ECC_WorldDynamic" "ECR_Block")
  (Collision|SetCollisionResponsetoChannel _sphere "ECC_Pawn" "ECR_Ignore"))

(fn SpawnStud
  (LocalVariables|SetRandomToSpawn (Math|Random|RandomInteger 10))
  (for _index (range 0 (LocalVariables|GetRandomToSpawn))
    (bind _returnvalue (Game|SpawnActorfromClass "/Game/Assets/Blueprints/Entity/Stud/BP_Stud.BP_Stud_C" (Transformation|GetWorldTransform (Variables|Default|GetSphere)) "AdjustIfPossibleButAlwaysSpawn" 0 0))
    (if (Math|Random|RandomBoolwithWeight 0.3)
      (Variables|/Game/Assets/Blueprints/Entity/Stud/BP_Stud.BP_Stud_C|SetTypeStud _returnvalue "NewEnumerator1"))))