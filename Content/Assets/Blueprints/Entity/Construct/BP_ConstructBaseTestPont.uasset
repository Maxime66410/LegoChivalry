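; Test construct actor, apparently a LEGO-style bridge ("Pont"), that assembles itself from loose pieces while building is active.
; BeginPlay caches piece meshes and transforms, then randomly scatters them with physics enabled.
; While Build is active and until CancelBuild, Tick disables physics and interpolates pieces sequentially toward saved transforms, each waiting for its predecessor.
; Placed pieces play random click sounds; completion plays a finish sound and is exposed through VerifyIsBuild.
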(event EventCancelBuild
  (Variables|Logic|SetIsBuild? false))

(event EventBuild
  (Variables|Logic|SetIsBuild? true))

(event EventBeginPlay
  (Setup|SetupConstruct)
  (Mechanic|DisorderPart))

(event EventTick
  (params (DeltaSeconds :type Float%20%28single-precision%29))
  (Variables|Logic|SetDelta%20Seconds DeltaSeconds)
  (Mechanic|PlacePart))

(fn ConstructionScript)

(fn SetupConstruct
  (Variables|Setup|SetArrayMesh (Utilities|SetupArrayMesh))
  (Variables|Setup|SetArrayLocationPiece (Utilities|SetupArrayTransform))
  (bind _o_array (Setup|SetupArrayBool))
  (Variables|Setup|SetArrayPartPlaced _o_array))

(fn DisorderPart
  (bind _returnvalue (Math|Random|RandomFloatinRange -5e+01 5e+01))
  (bind _returnvalue_2 (Math|Random|RandomFloatinRange -5e+01 5e+01))
  (bind _returnvalue_3 (Math|Random|RandomFloatinRange -5e+01 5e+01))
  (for _array_element (Variables|Setup|GetArrayMesh)
    (Transformation|SetRelativeLocation _array_element (Math|Vector|MakeVector _returnvalue_2 _returnvalue_3 _returnvalue) false false)
    (Transformation|SetRelativeRotation _array_element (Math|Rotator|MakeRotator _returnvalue_2 _returnvalue_3 _returnvalue) false false)
    (Physics|SetSimulatePhysics _array_element true)))

(fn SetupArrayBool
  (for _array_element (Variables|Setup|GetArrayMesh)
    (Utilities|Array|Add (LocalVariables|GetLocalArray) false))
  (return (LocalVariables|GetLocalArray)))

(fn PlacePart
  (if (Variables|Logic|GetIsBuild?)
    (if (not (Variables|Logic|GetCompleted))
      (for (_array_element _array_index) (Variables|Setup|GetArrayPartPlaced)
        (if (Variables|Logic|GetIsBuild?)
          (if (not _array_element)
            (if (== _array_index 0)
              (Transformation|SetRelativeTransform (Utilities|Array|Get(acopy) (Variables|Setup|GetArrayMesh) _array_index) (Class|KismetMathLibrary|TInterpto (Transformation|GetWorldTransform (Utilities|Array|Get(acopy) (Variables|Setup|GetArrayMesh) _array_index)) (Utilities|Array|Get(acopy) (Variables|Setup|GetArrayLocationPiece) _array_index) (Variables|Logic|GetDelta%20Seconds) (Variables|Logic|GetBuildSpeed)) false false)
              (Physics|SetSimulatePhysics (Utilities|Array|Get(acopy) (Variables|Setup|GetArrayMesh) _array_index) false)
              (if (Class|KismetMathLibrary|NearlyEqualTransformTransform (Transformation|GetWorldTransform (Utilities|Array|Get(acopy) (Variables|Setup|GetArrayMesh) _array_index)) (Class|KismetMathLibrary|TInterpto (Transformation|GetWorldTransform (Utilities|Array|Get(acopy) (Variables|Setup|GetArrayMesh) _array_index)) (Utilities|Array|Get(acopy) (Variables|Setup|GetArrayLocationPiece) _array_index) (Variables|Logic|GetDelta%20Seconds) (Variables|Logic|GetBuildSpeed)) 0.0001 0.0001 0.0001)
                (Utilities|Array|SetArrayElem (Variables|Setup|GetArrayPartPlaced) _array_index true)
                (Logic|PlaySound false))
              (elif (Utilities|Array|Get(acopy) (Variables|Setup|GetArrayPartPlaced) (- _array_index 1))
                (Transformation|SetRelativeTransform (Utilities|Array|Get(acopy) (Variables|Setup|GetArrayMesh) _array_index) (Class|KismetMathLibrary|TInterpto (Transformation|GetWorldTransform (Utilities|Array|Get(acopy) (Variables|Setup|GetArrayMesh) _array_index)) (Utilities|Array|Get(acopy) (Variables|Setup|GetArrayLocationPiece) _array_index) (Variables|Logic|GetDelta%20Seconds) (Variables|Logic|GetBuildSpeed)) false false)
                (Physics|SetSimulatePhysics (Utilities|Array|Get(acopy) (Variables|Setup|GetArrayMesh) _array_index) false)
                (if (Class|KismetMathLibrary|NearlyEqualTransformTransform (Transformation|GetWorldTransform (Utilities|Array|Get(acopy) (Variables|Setup|GetArrayMesh) _array_index)) (Class|KismetMathLibrary|TInterpto (Transformation|GetWorldTransform (Utilities|Array|Get(acopy) (Variables|Setup|GetArrayMesh) _array_index)) (Utilities|Array|Get(acopy) (Variables|Setup|GetArrayLocationPiece) _array_index) (Variables|Logic|GetDelta%20Seconds) (Variables|Logic|GetBuildSpeed)) 0.0001 0.0001 0.0001)
                  (Utilities|Array|SetArrayElem (Variables|Setup|GetArrayPartPlaced) _array_index true)
                  (Logic|PlaySound false)))))))
      (bind _array_element_2 (Utilities|Array|ForEachLoopwithBreak (Variables|Setup|GetArrayPartPlaced) :!label _label)
        (:LoopBody
          (if (not _array_element_2)
            (LocalVariables|SetAllIsBuild false)
            (goto _label Break)))
        (:Completed
          (if (LocalVariables|GetAllIsBuild)
            (Variables|Logic|SetCompleted true)
            (Logic|PlaySound true)))))))

(fn PlaySound
  (params (Finish%20? :type Boolean))
  (if Finish%20?
    (Audio|PlaySound2D "/Game/Assets/Audio/Build/Build/SW_Lego-building-finish-sfx.SW_Lego-building-finish-sfx" 1.0 1.0 0.0 0 0)
    (else
      (Audio|PlaySound2D (Utilities|Select :Index (Math|Random|RandomIntegerinRange 0 5) :Option%200 "/Game/Assets/Audio/Build/Build/SW_LEGO_FORM_1.SW_LEGO_FORM_1" :Option%201 "/Game/Assets/Audio/Build/Build/SW_LEGO_FORM_2.SW_LEGO_FORM_2" :Option%202 "/Game/Assets/Audio/Build/Build/SW_LEGO_FORM_3.SW_LEGO_FORM_3" :Option%203 "/Game/Assets/Audio/Build/Build/SW_LEGO_FORM_4.SW_LEGO_FORM_4" :Option%204 "/Game/Assets/Audio/Build/Build/SW_LEGO_FORM_5.SW_LEGO_FORM_5" :Option%205 "/Game/Assets/Audio/Build/Build/SW_LEGO_FORM_6.SW_LEGO_FORM_6") 1.0 1.0 0.0 0 0))))

(fn VerifyIsBuild
  (return (Variables|Logic|GetCompleted)))