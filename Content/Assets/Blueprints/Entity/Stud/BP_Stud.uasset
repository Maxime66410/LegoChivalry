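; Collectible Lego stud pickup in four tiers (silver, gold, blue, purple) that set its material, point value and sound.
; Tick spins the mesh; after three seconds physics simulation stops and it eases slightly above its last height.
; On player overlap it removes the mesh, triggers the player's UI, adds points through GM_LegoMode, plays a sound and destroys itself.
; A self-restarting timer reapplies the material every second.
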(event OnComponentBeginOverlap(StudStaticMesh)
  (params (OverlappedComponent :type Primitive%20Component%20Object%20Reference) (OtherActor :type Actor%20Object%20Reference) (OtherComp :type Primitive%20Component%20Object%20Reference) (OtherBodyIndex :type Integer) (bFromSweep :type Boolean) (SweepResult :type Hit%20Result%20Structure%20%28by%20ref%29))
  (bind _asbp_player (Utilities|Casting|CastToBP_Player OtherActor))
  (Components|DestroyComponent (Variables|Default|GetStudStaticMesh))
  (Default|PlayGetStud (Variables|/Game/Assets/Blueprints/Players/BP_Player.BP_Player_C|GetUI_Game _asbp_player) (Variables|Default|GetTypeStud))
  (CallFunction|GetItem)
  (CallFunction|PlaySound)
  (Utilities|FlowControl|Delay 1.0)
  (Actor|DestroyActor))

(event Custom|VerifyStatus
  (CallFunction|SetupMaterial)
  (Utilities|Time|SetTimerbyEvent (delegate Custom|VerifyStatus) 1.0))

(event EventTick
  (params (DeltaSeconds :type Float%20%28single-precision%29))
  (Variables|Default|SetDelta%20Seconds DeltaSeconds)
  (CallFunction|RotateStup)
  (CallFunction|FreezePosition))

(event EventBeginPlay
  (CallFunction|SetupMaterial)
  (CallFunction|SetupGM)
  (Utilities|Time|SetTimerbyFunctionName 0 "StopRandomMovement" 3.0)
  (CallFunction|VerifyStatus))

(fn ConstructionScript)

(fn RotateStup
  (bind _studstaticmesh (Variables|Default|GetStudStaticMesh))
  (Utilities|IsValid _studstaticmesh
    (:Is%20Valid
      (Transformation|SetWorldRotation _studstaticmesh (Math|Rotator|MakeRotator 8e+01 0.0 (+ (.yaw (Transformation|GetWorldRotation _studstaticmesh)) -3.5)) false false))))

(fn SetupMaterial
  (bind _studstaticmesh (Variables|Default|GetStudStaticMesh))
  (Utilities|IsValid _studstaticmesh
    (:Is%20Valid
      (switch Utilities|FlowControl|Switch|SwitchonE_StudType (Variables|Default|GetTypeStud)
        (:NewEnumerator0
          (Rendering|Material|SetMaterial _studstaticmesh 0 "/Game/Assets/Materials/Stud/M_Stud_Silver.M_Stud_Silver"))
        (:NewEnumerator1
          (Rendering|Material|SetMaterial _studstaticmesh 0 "/Game/Assets/Materials/Stud/M_Stud_Gold.M_Stud_Gold"))
        (:NewEnumerator2
          (Rendering|Material|SetMaterial _studstaticmesh 0 "/Game/Assets/Materials/Stud/M_Stud_Blue.M_Stud_Blue"))
        (:NewEnumerator3
          (Rendering|Material|SetMaterial _studstaticmesh 0 "/Game/Assets/Materials/Stud/M_Stud_Purple.M_Stud_Purple"))))))

(fn SetupGM
  (bind _asgm_lego_mode (Utilities|Casting|CastToGM_LegoMode (Game|GetGameMode)))
  (Variables|Default|SetAs%20GM%20Lego%20Mode _asgm_lego_mode))

(fn GetItem
  (Utilities|IsValid (Variables|Default|GetAs%20GM%20Lego%20Mode)
    (:Is%20Valid
      (Default|AddStud (Variables|Default|GetAs%20GM%20Lego%20Mode) (Utilities|Select :Index (Variables|Default|GetTypeStud) :NewEnumerator0 10 :NewEnumerator1 100 :NewEnumerator2 1000 :NewEnumerator3 10000)))
    (:Is%20Not%20Valid
      (Development|PrintString "ERROR : Gamemode \"GM_LegoMode\" is not SET" true true "(R=1.000000,G=0.961340,B=0.000000,A=1.000000)"))))

(fn PlaySound
  (bind _returnvalue (Math|Random|RandomIntegerinRange 0 5))
  (bind _returnvalue_2 (Utilities|Select :Index _returnvalue :Option%200 "/Game/Assets/Audio/Stud/SW_StudSilver.SW_StudSilver" :Option%201 "/Game/Assets/Audio/Stud/SW_StudSilver1.SW_StudSilver1" :Option%202 "/Game/Assets/Audio/Stud/SW_StudSilver2.SW_StudSilver2" :Option%203 "/Game/Assets/Audio/Stud/SW_StudSilver3.SW_StudSilver3" :Option%204 "/Game/Assets/Audio/Stud/SW_StudSilver4.SW_StudSilver4" :Option%205 "/Game/Assets/Audio/Stud/SW_StudSilver5.SW_StudSilver5"))
  (Audio|PlaySound2D (Utilities|Select :Index (Variables|Default|GetTypeStud) :NewEnumerator0 _returnvalue_2 :NewEnumerator1 _returnvalue_2 :NewEnumerator2 "/Game/Assets/Audio/Stud/SW_StudBlue.SW_StudBlue" :NewEnumerator3 "/Game/Assets/Audio/Stud/SW_StudPurple.SW_StudPurple") 1.0 1.0 0.0 0 0))

(fn StopRandomMovement
  (bind _studstaticmesh (Variables|Default|GetStudStaticMesh))
  (Utilities|IsValid _studstaticmesh
    (:Is%20Valid
      (Physics|SetSimulatePhysics _studstaticmesh false)
      (Variables|Default|SetCanFreeze true))))

(fn FreezePosition
  (bind _studstaticmesh (Variables|Default|GetStudStaticMesh))
  (bind _studstaticmesh_2 (Variables|Default|GetStudStaticMesh))
  (bind _relativelocation (Variables|/Script/Engine.SceneComponent|GetRelativeLocation _studstaticmesh_2))
  (if (Variables|Default|GetCanFreeze)
    (Utilities|IsValid _studstaticmesh_2
      (:Is%20Valid
        (Transformation|SetRelativeLocation _studstaticmesh_2 (Math|Vector|MakeVector (.x _relativelocation) (.y _relativelocation) (Math|Interpolation|FInterpTo (.z _relativelocation) (+ (Variables|Default|GetLastPosZ) 5.0) (Variables|Default|GetDelta%20Seconds) 1.0)) false false)))
    (else
      (Utilities|IsValid _studstaticmesh
        (:Is%20Valid
          (Variables|Default|SetLastPosZ (.z (Variables|/Script/Engine.SceneComponent|GetRelativeLocation _studstaticmesh))))))))