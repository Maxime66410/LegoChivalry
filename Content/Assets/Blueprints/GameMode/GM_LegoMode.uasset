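; GM_LegoMode is a game mode that keeps the stud score for a Lego-style game.
; AddStud and RemoveStud events raise or lower StudScore by a given count.
; Tick prints the current score to the screen every frame with a near-zero duration, acting as a debug readout.
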(event Custom|AddStud
  (params (Count :type Integer))
  ;[1 1 1] Add Stud
  (Variables|Default|SetStudScore (+ (Variables|Default|GetStudScore) Count)))

(event Custom|RemoveStud
  (params (Count :type Integer))
  ;[1 1 1] Remove Stud
  (Variables|Default|SetStudScore (- (Variables|Default|GetStudScore) Count)))

(event EventTick
  (params (DeltaSeconds :type Float%20%28single-precision%29))
  (Development|PrintString (Utilities|String|ToString(Integer) (Variables|Default|GetStudScore)) true true "(R=0.000000,G=0.660000,B=1.000000,A=1.000000)" 0.0001))

(fn ConstructionScript)