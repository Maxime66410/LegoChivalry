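; BP_Minikit is a collectible minikit pickup that spins around its yaw each tick.
; When a BP_Player overlaps it while not flagged invisible, it adds one to the GM_LegoMode count, triggers the player's UI animation and pickup sound, then destroys itself.
; Instances flagged IsInvisible start hidden, silent and without collision; the Enable event reveals them with an appear sound and restored collision, but leaves that flag unchanged.
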(event OnComponentBeginOverlap(StaticMesh)
  (params (OverlappedComponent :type Primitive%20Component%20Object%20Reference) (OtherActor :type Actor%20Object%20Reference) (OtherComp :type Primitive%20Component%20Object%20Reference) (OtherBodyIndex :type Integer) (bFromSweep :type Boolean) (SweepResult :type Hit%20Result%20Structure%20%28by%20ref%29))
  (bind _as_gm_lego_mode (Variables|Default|GetAs%20GM%20Lego%20Mode))
  ;[1 1 1] Get items
  (bind _asbp_player (Utilities|Casting|CastToBP_Player OtherActor))
  (if (not (Variables|Default|GetIsInvisible?))
    (Utilities|IsValid _as_gm_lego_mode
      (:Is%20Valid
        (Default|AddMK _as_gm_lego_mode 1)
        (Default|PlayGetMK (Variables|/Game/Assets/Blueprints/Players/BP_Player.BP_Player_C|GetUI_Game _asbp_player))
        (Audio|PlaySound2D "/Game/Assets/Audio/Stud/Special/SW_MK-PICKUP.SW_MK-PICKUP" 1.0 1.0 0.0 0 0)
        (Components|DestroyComponent (Variables|Default|GetStaticMesh))
        (Utilities|FlowControl|Delay 1.0)
        (Actor|DestroyActor)))))

(event Custom|Enable
  (bind _staticmesh (Variables|Default|GetStaticMesh))
  ;[1 1 1] Reppear
  (Audio|PlaySound2D "/Game/Assets/Audio/Stud/Special/SW_MK-APPEAR.SW_MK-APPEAR" 1.0 1.0 0.0 0 0)
  (Rendering|SetVisibility _staticmesh true false)
  (Collision|SetCollisionEnabled _staticmesh "QueryAndPhysics")
  (Audio|Components|Audio|Play (Variables|Default|GetSFX) 0.0))

(event EventTick
  (params (DeltaSeconds :type Float%20%28single-precision%29))
  ;[1 1 1] Animations
  (Variables|Default|SetDelta%20Seconds DeltaSeconds)
  (CallFunction|RotateObject))

(event EventBeginPlay
  ;[1 1 1] Start
  (CallFunction|GetGM)
  (CallFunction|CheckifEnabled?))

(fn ConstructionScript)

(fn RotateObject
  (bind _staticmesh (Variables|Default|GetStaticMesh))
  (bind _relativerotation (Variables|/Script/Engine.SceneComponent|GetRelativeRotation _staticmesh))
  (Utilities|IsValid _staticmesh
    (:Is%20Valid
      (Transformation|SetRelativeRotation _staticmesh (Math|Rotator|MakeRotator 0.0 0.0 (Math|Interpolation|FInterpTo (.yaw _relativerotation) (+ (.yaw _relativerotation) 1e+02) (Variables|Default|GetDelta%20Seconds) 1.0)) false false))))

(fn CheckifEnabled?
  (bind _staticmesh (Variables|Default|GetStaticMesh))
  (if (Variables|Default|GetIsInvisible?)
    (Rendering|SetVisibility _staticmesh false false)
    (Collision|SetCollisionEnabled _staticmesh "NoCollision")
    (Audio|Components|Audio|Stop (Variables|Default|GetSFX))))

(fn GetGM
  (bind _asgm_lego_mode (Utilities|Casting|CastToGM_LegoMode (Game|GetGameMode)))
  (Variables|Default|SetAs%20GM%20Lego%20Mode _asgm_lego_mode))