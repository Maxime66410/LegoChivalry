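; BP_Heart is a health pickup that heals BP_Player when touched.
; Each Tick, RotateObject spins the static mesh on yaw by interpolating toward a moving offset ahead of its current angle.
; On mesh overlap, a player below full health gains life, sees the heart UI feedback and hears a sound.
; The mesh is destroyed immediately, and the actor follows after a short delay.
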(event OnComponentBeginOverlap(StaticMesh)
  (params (OverlappedComponent :type Primitive%20Component%20Object%20Reference) (OtherActor :type Actor%20Object%20Reference) (OtherComp :type Primitive%20Component%20Object%20Reference) (OtherBodyIndex :type Integer) (bFromSweep :type Boolean) (SweepResult :type Hit%20Result%20Structure%20%28by%20ref%29))
  (bind _asbp_player (Utilities|Casting|CastToBP_Player OtherActor))
  (if (<= (Variables|/Game/Assets/Blueprints/Players/BP_Player.BP_Player_C|GetHealth _asbp_player) 99.9)
    (Default|AddLife _asbp_player 15.0)
    (Default|PlayGetHeart (Variables|/Game/Assets/Blueprints/Players/BP_Player.BP_Player_C|GetUI_Game _asbp_player))
    (Components|DestroyComponent (Variables|Default|GetStaticMesh))
    (Audio|PlaySound2D "/Game/Assets/Audio/Player/Heart/SW_HEART.SW_HEART" 1.0 1.0 0.0 0 0)
    (Utilities|FlowControl|Delay 1.0)
    (Actor|DestroyActor)))

(event EventTick
  (params (DeltaSeconds :type Float%20%28single-precision%29))
  (Variables|Default|SetDelta%20Seconds DeltaSeconds)
  (CallFunction|RotateObject))

(fn ConstructionScript)

(fn RotateObject
  (bind _staticmesh (Variables|Default|GetStaticMesh))
  (bind _relativerotation (Variables|/Script/Engine.SceneComponent|GetRelativeRotation _staticmesh))
  (Utilities|IsValid _staticmesh
    (:Is%20Valid
      (Transformation|SetRelativeRotation _staticmesh (Math|Rotator|MakeRotator 0.0 0.0 (Math|Interpolation|FInterpTo (.yaw _relativerotation) (+ (.yaw _relativerotation) 1e+02) (Variables|Default|GetDelta%20Seconds) 1.0)) false false))))