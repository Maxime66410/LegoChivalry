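; BP_FireMultiple is a fire zone that deals periodic damage to every actor inside its trigger box.
; Overlap begin and end events add and remove actors from a tracked array, with a check against duplicate entries.
; A looping one-second timer started at BeginPlay calls TakeDamage, which applies fixed damage to each valid tracked actor and force-disables the shield of any BP_Player first.
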(event OnComponentBeginOverlap(TriggerBox)
  (params (OverlappedComponent :type Primitive%20Component%20Object%20Reference) (OtherActor :type Actor%20Object%20Reference) (OtherComp :type Primitive%20Component%20Object%20Reference) (OtherBodyIndex :type Integer) (bFromSweep :type Boolean) (SweepResult :type Hit%20Result%20Structure%20%28by%20ref%29))
  (CallFunction|AddActor OtherActor))

(event OnComponentEndOverlap(TriggerBox)
  (params (OverlappedComponent :type Primitive%20Component%20Object%20Reference) (OtherActor :type Actor%20Object%20Reference) (OtherComp :type Primitive%20Component%20Object%20Reference) (OtherBodyIndex :type Integer))
  (CallFunction|RemoveActor OtherActor))

(event EventBeginPlay
  (Utilities|Time|SetTimerbyFunctionName 0 "TakeDamage" 1.0 true))

(fn ConstructionScript)

(fn AddActor
  (params (Actor :type Actor%20Object%20Reference))
  (bind _arrayactor (Variables|Default|GetArrayActor))
  (bind _array_element (Utilities|Array|ForEachLoopwithBreak _arrayactor :!label _label)
    (:LoopBody
      (if (== _array_element Actor)
        (LocalVariables|SetIsNotIn false)
        (goto _label Break)))
    (:Completed
      (if (LocalVariables|GetIsNotIn)
        (Utilities|Array|Add _arrayactor Actor)))))

(fn RemoveActor
  (params (Actor :type Actor%20Object%20Reference))
  (bind _arrayactor (Variables|Default|GetArrayActor))
  (bind (_array_element _array_index) (Utilities|Array|ForEachLoopwithBreak _arrayactor :!label _label)
    (:LoopBody
      (if (== _array_element Actor)
        (LocalVariables|SetIstIn true)
        (LocalVariables|SetLocalRemoveIndex _array_index)
        (goto _label Break)))
    (:Completed
      (if (LocalVariables|GetIstIn)
        (Utilities|Array|RemoveIndex _arrayactor (LocalVariables|GetLocalRemoveIndex))))))

(fn TakeDamage
  (bind _arrayactor (Variables|Default|GetArrayActor))
  (if (Utilities|Array|IsNotEmpty _arrayactor)
    (for _array_element _arrayactor
      (Utilities|IsValid _array_element
        (:Is%20Valid
          (bind _asbp_player (Utilities|Casting|CastToBP_Player _array_element)
            (:then
              (Default|ForceDisabledShield _asbp_player))
            (:CastFailed
              _))
          (Game|Damage|ApplyDamage _array_element 5.0 0 self))))))